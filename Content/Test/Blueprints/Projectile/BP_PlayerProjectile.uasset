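; BP_PlayerProjectile is the player's projectile, which damages flying enemies on contact.
; When its ProjectileCollision component begins an overlap, it casts the other actor to BP_EnemyFlyingPawn and ignores anything else.
; On a match it applies ProjectileDamage, with its owner as damage causer, then destroys itself.
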(event `self.ReceiveBeginPlay`
  (`parent.ReceiveBeginPlay`))

(event `self.ProjectileCollision.OnComponentBeginOverlap`
  (params (OverlappedComponent :type "PrimitiveComponent Object Reference") (OtherActor :type "Actor Object Reference") (OtherComp :type "PrimitiveComponent Object Reference") (OtherBodyIndex :type Integer) (bFromSweep :type Boolean) (SweepResult :type "HitResult Structure (by ref)"))
  ;[1 1 1] 如果玩家的抛射物击中敌人，则执行造成伤害后销毁
  (bind _asbp_enemy_flying_pawn (cast `/Game/Test/Blueprints/Pawns/Enemy/BP_EnemyFlyingPawn` OtherActor))
  (`GameplayStatics.ApplyDamage` _asbp_enemy_flying_pawn (`self.ProjectileDamage`) null (`self.GetOwner`))
  (`self.K2_DestroyActor`))

(fn `UserConstructionScript`
  (`parent.UserConstructionScript`))