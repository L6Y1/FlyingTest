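; Game State for a flying game that tracks how many enemies have been destroyed.
; On BeginPlay it resets the count and fetches the total enemy count from the Game Mode through a message call.
; AddEnemyDestroyedNum increases the count and fires the OnEnemyAllDistroyed dispatcher when it exactly equals that total.
; A getter exposes the count, and Tick prints it on screen every frame.
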(event `self.ReceiveBeginPlay`
  (`self.ResetGameState`))

(event `self.ReceiveTick`
  (params (DeltaSeconds :type "Float (single-precision)"))
  (`KismetSystemLibrary.PrintString` (`KismetStringLibrary.Conv_IntToString` (`self.DestroyedEnemyNum`)) true false (struct :`G` 0.66 :`B` 1.0 :`A` 1.0) 0.0))

(event `self.AddEnemyDestroyedNum`
  (params (AddNum :type Integer))
  ;[1 1 1] 增加得分
  (bind _output_get (set `self.DestroyedEnemyNum` (+ AddNum (`self.DestroyedEnemyNum`))))
  ;;[0.6135 1 0.5758] 如果消灭敌人数和应生成敌人总数相等，则触发所有事件派发器
  (if (== _output_get (`self.TotalEnemyNum`))
    (`self.OnEnemyAllDistroyed`)))

(event `self.ResetGameState`
  ;[1 1 1] 重设得分，并从游戏模式中获取应该生成敌人的总个数
  (set `self.DestroyedEnemyNum` 0)
  (bind _totalenemynum (message `/Game/Test/Blueprints/Utils/Interface/BP_FlyingGameModeInterface.GetTotalEnemyNum` (`GameplayStatics.GetGameMode`)))
  (set `self.TotalEnemyNum` _totalenemynum))

(fn `GetEnemyDestroyedNum`
  (returns (EnemyDestroyedNum :type Integer))
  (return (`self.DestroyedEnemyNum`)))

(fn `UserConstructionScript`)