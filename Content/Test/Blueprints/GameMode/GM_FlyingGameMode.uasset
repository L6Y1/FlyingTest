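; Game mode for a flying shooter that runs each round's enemy spawning and difficulty level.
; ResetGame reads the enemy quota from the current difficulty setting, resets GameState stats, rebuilds the controller's UI and binds player death to stop spawning.
; A looping timer spawns enemies at random free locations until the quota is met, skipping ticks when none are free.
; Locations move between free and occupied arrays, with an event to release them.
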(event `self.ReceiveBeginPlay`
  ;[1 1 1] 第一次进入游戏时也相当于重新游玩
  (`self.ResetGame`))

(event `self.FreeOccupiedLocation`
  (params (InVector :type "Vector Structure"))
  ;[1 1 1] 将所给的向量加入未占用位置数组中
  (`KismetArrayLibrary.Array_AddUnique` (`self.EnemySpawnLocationArray`) InVector)
  (`KismetArrayLibrary.Array_RemoveItem` (`self.EnemyAlreadySpawnedLocationArray`) InVector))

(event `self.ToHigherDifficulty`
  ;[1 1 1] 进入更高难度，如果难度已经为最高则保持最高难度
  (if (< (`self.CurrentDifficultyLevel`) (`KismetArrayLibrary.Array_Length` (`self.ProjectileDamageSetting`)))
    (`/Engine/EditorBlueprintResources/StandardMacros.IncrementInt` (`self.CurrentDifficultyLevel`))))

(event `self.ResetGame`
  (bind (_output_playerprojectiledamage _output_enemyprojectiledamage _output_totalenemynum) (break `/Game/Test/Blueprints/Utils/Structure/S_DifficultySettingStructure` (`|GetArrayItem` (`self.ProjectileDamageSetting`) (`self.CurrentDifficultyLevel`))))
  ;[1 1 1] 重设游戏
  ;;[0.6135 1 0.5758] 已生成的敌人设置为0
  (set `self.SpawnedEnemyNum` 0)
  ;;[0.6135 1 0.5758] 根据难度设置要生成的敌人数量
  (set `self.TotalEnemyNum` _output_totalenemynum)
  ;;[0.6135 1 0.5758] 启动定时器生成敌人
  (`self.StartTimerToSpawnEnemyRandomly`)
  ;;[0.6135 1 0.5758] 当玩家死亡后停止生成敌人
  (add `/Game/Test/Blueprints/Pawns/Player/BP_PlayerFlyingPawn.OnPlayerDestroyed` (cast `/Game/Test/Blueprints/Pawns/Player/BP_PlayerFlyingPawn` (`Controller.K2_GetPawn` (`GameplayStatics.GetPlayerController` 0)) :!pure true) (`|CreateDelegate` :!event `StopSpawningEnemyTimer`))
  ;;[0.6135 1 0.5758] 重设游戏状态中的消灭敌人数
  (message `/Game/Test/Blueprints/Utils/Interface/BP_FlyingGamestateInterface.ResetGameState` (`GameplayStatics.GetGameState`))
  ;;[0.6135 1 0.5758] 重设玩家控制器中的UI
  (`/Game/Test/Blueprints/Controller/BP_FlyingPlayerController.ConstructMainUI` (cast `/Game/Test/Blueprints/Controller/BP_FlyingPlayerController` (`GameplayStatics.GetPlayerController` 0) :!pure true)))

(fn `AddVectorToEnemySpawnLocationArray`
  (params (InVector :type "Vector Structure"))
  (returns (AddSuccess :type Boolean))
  ;[1 1 1] 将指定的向量添加到敌人生成地点数组中
  (`KismetArrayLibrary.Array_AddUnique` (`self.EnemySpawnLocationArray`) InVector)
  (return true))

(fn `DeleteVectorInEnemySpawnLocationArray`
  (params (InVector :type "Vector Structure"))
  (returns (DeleteSuccess :type Boolean))
  ;[1 1 1] 将指定的向量从敌人生成地点数组中删除
  (bind _returnvalue (`KismetArrayLibrary.Array_RemoveItem` (`self.EnemySpawnLocationArray`) InVector))
  (return _returnvalue))

(fn `GetCurrentDifficultySetting`
  (returns (DifficultySetting :type "/Game/Test/Blueprints/Utils/Structure/S_DifficultySettingStructure Structure"))
  (return (`|GetArrayItem` (`self.ProjectileDamageSetting`) (`self.CurrentDifficultyLevel`))))

(fn `GetTotalEnemyNum`
  (returns (TotalEnemyNum :type Integer))
  (return (`self.TotalEnemyNum`)))

(fn `SpawnEnemyRandomly`
  (locals (SpawningLocation :type "Vector Structure"))
  ;[1 1 1] 如果没有生成完预定数量的敌人则继续生成，反之则停止定时器
  (if (< (`self.SpawnedEnemyNum`) (`self.TotalEnemyNum`))
    ;[1 1 1] 场内没有空位时则本周期不生成
    (if (`KismetArrayLibrary.Array_IsValidIndex` (`self.EnemySpawnLocationArray`))
      (set `local.SpawningLocation` (`KismetArrayLibrary.Array_Random` (`self.EnemySpawnLocationArray`)))
      (`KismetArrayLibrary.Array_AddUnique` (`self.EnemyAlreadySpawnedLocationArray`) (`local.SpawningLocation`))
      (`|SpawnActorFromClass` "/Game/Test/Blueprints/Pawns/Enemy/BP_EnemyFlyingPawn.BP_EnemyFlyingPawn_C" (`KismetMathLibrary.MakeTransform` (`local.SpawningLocation`) (struct) (3.0 3.0 3.0)) "Undefined" "OverrideRootScale" null null)
      ;[1 1 1] 生成后在未占用位置数组中删除相应坐标
      (`KismetArrayLibrary.Array_RemoveItem` (`self.EnemySpawnLocationArray`) (`local.SpawningLocation`))
      (`/Engine/EditorBlueprintResources/StandardMacros.IncrementInt` (`self.SpawnedEnemyNum`)))
    (else
      (`self.StopSpawningEnemyTimer`))))

(fn `StartTimerToSpawnEnemyRandomly`
  (`self.SpawnEnemyRandomly`)
  (bind _returnvalue (`KismetSystemLibrary.K2_SetTimerDelegate` (`|CreateDelegate` :!event `SpawnEnemyRandomly`) 3.0 true))
  (set `self.SpawnEnemyRandomlyHandle` _returnvalue))

(fn `StopSpawningEnemyTimer`
  (`KismetSystemLibrary.K2_ClearAndInvalidateTimerHandle` (`self.SpawnEnemyRandomlyHandle`)))

(fn `UserConstructionScript`)