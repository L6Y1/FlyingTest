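; Player controller for a flying combat mission that handles firing and UI.
; On BeginPlay it shows the main HUD; left click tells the possessed BP_PlayerFlyingPawn to spawn a projectile.
; On possess it binds to the pawn's destroyed and the game state's all-enemies-destroyed dispatchers to raise end-of-mission UI.
; ConstructMissionUI picks success or failure by whether a pawn is still controlled, then switches to UI-only input with a cursor.
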(event `self.ReceiveBeginPlay`
  (`self.ConstructMainUI`))

(event `self.ReceivePossess`
  (params (PossessedPawn :type "Pawn Object Reference"))
  (bind _asbp_player_flying_pawn (cast `/Game/Test/Blueprints/Pawns/Player/BP_PlayerFlyingPawn` PossessedPawn :!pure true))
  (`/Engine/EditorBlueprintResources/StandardMacros.IsValid` _asbp_player_flying_pawn
    (:`Is Valid`
      (set `self.ControllingPawn` _asbp_player_flying_pawn)
      ;[1 1 1] 绑定事件到玩家pawn中的事件派发器，玩家被摧毁时调用
      (add `/Game/Test/Blueprints/Pawns/Player/BP_PlayerFlyingPawn.OnPlayerDestroyed` _asbp_player_flying_pawn (`|CreateDelegate` :!event `ConstructMissionUI`))
      ;[1 1 1] 绑定事件到游戏状态中的事件派发器，所有敌人被摧毁后调用
      (add `/Game/Test/Blueprints/GameState/BP_FlyingGameState.OnEnemyAllDistroyed` (cast `/Game/Test/Blueprints/GameState/BP_FlyingGameState` (`GameplayStatics.GetGameState`) :!pure true) (`|CreateDelegate` :!event `ConstructMissionUI`)))))

(event `Key|LeftMouseButton`
  (params (Key :type "Key Structure"))
  (:`Pressed`
    (`/Game/Test/Blueprints/Pawns/BP_FlyingPawnBase.SpawnProjectile` (`self.ControllingPawn`))))

(fn `ConstructMainUI`
  (bind _returnvalue (`|CreateWidget` "/Game/Test/Blueprints/UI/Player/BP_PlayerMainWidget.BP_PlayerMainWidget_C"))
  (`UserWidget.AddToViewport` _returnvalue 0))

(fn `ConstructMissionUI`
  (`WidgetLayoutLibrary.RemoveAllWidgets`)
  (bind _returnvalue (`|CreateWidget` (select `bool` (`KismetSystemLibrary.IsValid` (`self.K2_GetPawn`)) :`false` "/Game/Test/Blueprints/UI/Mission/BP_MissionFailWidget.BP_MissionFailWidget_C" :`true` "/Game/Test/Blueprints/UI/Mission/BP_MissionSuccessWidget.BP_MissionSuccessWidget_C" :!type "UserWidget Class Reference")))
  (`UserWidget.AddToViewport` _returnvalue 0)
  (`WidgetBlueprintLibrary.SetInputMode_UIOnlyEx` self null)
  (set `self.bShowMouseCursor` true))

(fn `UserConstructionScript`)